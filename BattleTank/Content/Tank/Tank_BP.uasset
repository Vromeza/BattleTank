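; Player tank Blueprint that routes input to track throttles, camera aiming and firing.
; On BeginPlay it passes its Barrel and Turret components to setter functions and sets a camera axis multiplier.
; Each track takes its own throttle axis, and the Fire action calls Fire.
; Aim axes orbit the camera, yawing an azimuth gimbal and pitching the spring arm separately, scaled by frame delta time.
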(event EventBeginPlay
  (Variables|Default|SetCameraAxisMultiplier 1e+01)
  (Class|Tank|SetBarrelReference (Variables|Default|GetBarrel))
  (Class|Tank|SetTurretReference (Variables|Default|GetTurret)))

(event Collision|EventActorBeginOverlap
  (params (OtherActor :type Actor%20Object%20Reference)))

(event EventTick
  (params (DeltaSeconds :type Float%20%28single-precision%29)))

(event Input|ActionEvents|InputActionFire
  (params (Key :type Key%20Structure :default "AnyKey"))
  ;[1 1 1] Input handles
  (:Pressed
    (Class|Tank|Fire)))

(event Input|AxisEvents|InputAxisAimAzimuth
  (params (AxisValue :type Float%20%28single-precision%29))
  ;[1 1 1] Input handles
  (Transformation|AddRelativeRotation (Variables|Default|GetAzimuth%20Gimbal) (Math|Rotator|MakeRotator 0.0 0.0 (* AxisValue (Utilities|Time|GetWorldDeltaSeconds) (Variables|Default|GetCameraAxisMultiplier))) false false))

(event Input|AxisEvents|InputAxisAimElevation
  (params (AxisValue :type Float%20%28single-precision%29))
  ;[1 1 1] Input handles
  (Transformation|AddLocalRotation (Variables|Default|GetSpringArm) (Math|Rotator|MakeRotator 0.0 (* AxisValue (Utilities|Time|GetWorldDeltaSeconds) (Variables|Default|GetCameraAxisMultiplier)) 0.0) false false))

(event Input|AxisEvents|InputAxisLeftTrackThrottle
  (params (AxisValue :type Float%20%28single-precision%29))
  (Class|TankTrack|SetThrottle (Variables|Default|GetLeftTrack) AxisValue))

(event Input|AxisEvents|InputAxisRightTrackThrottle
  (params (AxisValue :type Float%20%28single-precision%29))
  (Class|TankTrack|SetThrottle (Variables|Default|GetRightTrack) AxisValue))

(fn ConstructionScript)